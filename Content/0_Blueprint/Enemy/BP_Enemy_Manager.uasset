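; Enemy manager that periodically relocates the enemy near the player while IsSeingPlayer is false.
; A looping timer, tuned by the DAEnemyManager data, destroys every BP_Enemy and gathers BP_SpawnPoints within a min/max distance band around the player.
; One new enemy spawns at a random point from that set, or none if the set is empty.
; Debug spheres for the distance band are present but disconnected.
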(event Custom|Spawn%20Enemy
  (bind _da_enemy_manager (Variables|Default|GetDA_Enemy_Manager))
  (if (not (Variables|Default|GetisSeingPlayer))
    (bind _outactors (Actor|GetAllActorsOfClass "/Game/0_Blueprint/Enemy/BP_Enemy.BP_Enemy_C"))
    (for _array_element _outactors
      (Actor|DestroyActor _array_element))
    (Utilities|Array|Clear (Variables|Default|GetPossibleSpawns))
    (bind _outactors_2 (Actor|GetAllActorsOfClass "/Game/0_Blueprint/Enemy/BP_SpawnPoints.BP_SpawnPoints_C"))
    (for _array_element_2 _outactors_2
      (if (Math|Float|InRange(Float) (Math|Vector|Distance(Vector) (Transformation|GetActorLocation _array_element_2) (Transformation|GetActorLocation (Game|Player|GetPlayerPawn 0))) (Variables|/Game/0_Blueprint/Enemy/BPDA_Enemy_Manager.BPDA_Enemy_Manager_C|GetMinDistFromPlayer _da_enemy_manager) (Variables|/Game/0_Blueprint/Enemy/BPDA_Enemy_Manager.BPDA_Enemy_Manager_C|GetMaxDistFromPlayer _da_enemy_manager))
        (Utilities|Array|Add (Variables|Default|GetPossibleSpawns) _array_element_2)))
    (if (Utilities|Array|IsNotEmpty (Variables|Default|GetPossibleSpawns))
      (Game|SpawnActorfromClass "/Game/0_Blueprint/Enemy/BP_Enemy.BP_Enemy_C" (Math|Transform|MakeTransform (Transformation|GetActorLocation (.OutItem (Utilities|Array|Random (Variables|Default|GetPossibleSpawns))))) "AlwaysSpawn" "MultiplyWithRoot" 0 0))))

(event EventBeginPlay
  (Utilities|Time|SetTimerbyEvent (delegate Custom|Spawn%20Enemy) (Variables|/Game/0_Blueprint/Enemy/BPDA_Enemy_Manager.BPDA_Enemy_Manager_C|GetTimeBtwSpawn (Variables|Default|GetDA_Enemy_Manager)) true true))

(fn ConstructionScript)